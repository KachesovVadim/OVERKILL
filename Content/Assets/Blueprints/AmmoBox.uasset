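; AmmoBox is an ammo pickup that refills the player's current weapon when the player character overlaps it.
; On overlap with player 0's ThirdPersonCharacter, it casts CurrentWeapon to Weapon and sets TotalAmmo to a multiple of MaxAmmo, overwriting the old value rather than adding to it.
; It then plays a 2D pickup sound and destroys itself.
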(event Collision|EventActorBeginOverlap
  (params (OtherActor :type Actor%20Object%20Reference))
  (bind _returnvalue (Game|GetPlayerCharacter 0))
  (bind _asthird_person_character (Utilities|Casting|CastToThirdPersonCharacter _returnvalue))
  (bind _currentweapon (Variables|/Game/Assets/Blueprints/ThirdPersonCharacter.ThirdPersonCharacter_C|GetCurrentWeapon _asthird_person_character))
  (bind _asweapon (Utilities|Casting|CastToWeapon _currentweapon))
  (if (== OtherActor _asthird_person_character)
    (Variables|/Game/Assets/Blueprints/Weapons/Weapon.Weapon_C|SetTotalAmmo _asweapon (* (Variables|/Game/Assets/Blueprints/Weapons/Weapon.Weapon_C|GetMaxAmmo _asweapon) 10))
    (Audio|PlaySound2D "/Game/Assets/Sounds/Weapon/AmmoPickup.AmmoPickup" 1.0 1.0 0.0 0 0)
    (Actor|DestroyActor)))

(fn ConstructionScript)