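; Spawner controller that populates the level with zombies and, optionally, ammo boxes at randomly chosen Spawner_ actors.
; After a short startup delay, SelectedSpawn re-calls itself every SpawnDuration, telling a random spawner to spawn a zombie until the total reaches MaxEnemies.
; If SpawnAmmoBoxes is set, a looping timer periodically spawns an AmmoBox at a random spawner's location.
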(event Custom|SelectedSpawn
  (bind _output_get (Variables|Default|SetSpawnedEnemies (+ (Variables|Default|GetSpawnedEnemies) 1)))
  (if (not (> _output_get (Variables|Default|GetMaxEnemies)))
    (bind _outactors (Actor|GetAllActorsOfClass "/Game/Assets/Blueprints/Spawner_.Spawner__C"))
    (Default|Spawn (Utilities|Array|Get(acopy) _outactors (Math|Random|RandomInteger (Utilities|Array|Length _outactors))) "/Game/Assets/Blueprints/Enemies/Zombie.Zombie_C")
    (Utilities|FlowControl|Delay (Variables|Default|GetSpawnDuration))
    (CallFunction|SelectedSpawn)))

(event EventBeginPlay
  (Utilities|FlowControl|Delay 0.3)
  (if (Variables|Default|GetSpawnAmmoBoxes)
    (Utilities|Time|SetTimerbyFunctionName 0 "SpawnAmmoBox" 6e+01 true))
  (CallFunction|SelectedSpawn))

(fn ConstructionScript)

(fn SpawnAmmoBox
  (bind _outactors (Actor|GetAllActorsOfClass "/Game/Assets/Blueprints/Spawner_.Spawner__C"))
  (Game|SpawnActorfromClass "/Game/Assets/Blueprints/AmmoBox.AmmoBox_C" (Math|Transform|MakeTransform (Transformation|GetActorLocation (Utilities|Array|Get(acopy) _outactors (Math|Random|RandomInteger (Utilities|Array|Length _outactors))))) "Undefined" 0 0))