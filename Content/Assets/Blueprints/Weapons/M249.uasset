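; M249 light machine gun weapon Blueprint, a child that inherits shooting from its parent weapon class.
; The construction script runs the parent's, then sets the gun's ammo, range, spread, damage, fire rate, knockback, automatic fire mode and firing and empty sounds.
; The Shoot event only calls the parent implementation, and GetSocket returns a socket's location, rotation and name from the M249 mesh along with the mesh reference.
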(event EventShoot
  (|CallParentFunction))

(fn ConstructionScript
  (|CallParentFunction)
  (bind _output_get (Variables|Default|SetMaxAmmo 100))
  (Variables|Default|SetCurrentAmmo _output_get)
  (Variables|Default|SetMaxDistance 7500)
  (Variables|Default|SetSpread 300)
  (Variables|Default|SetDamage 0.3)
  (Variables|Default|SetFireRate 0.06)
  (Variables|Default|SetKnockback -0.5)
  (Variables|Default|SetFireMode 0) ; 0 - Automatic, 1 - Semi Automatic
  (Variables|Default|SetSoundShoot "/Game/Assets/Sounds/Weapon/M249_Shoot.M249_Shoot")
  (Variables|Default|SetSoundNotShoot "/Game/Assets/Sounds/Weapon/Empty.Empty"))

(fn GetSocket
  (params (Socket :type Name :default "None"))
  (bind _m249 (Variables|Default|GetM249))
  (return (Transformation|GetSocketLocation _m249 Socket) (Transformation|GetSocketRotation _m249 Socket) Socket _m249))