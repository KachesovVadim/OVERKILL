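; AK74 weapon Blueprint, a child of a parent weapon class, configured as an automatic rifle.
; Its construction script runs the parent's, then sets ammo, range, spread, damage, fire rate, knockback, fire mode and sounds.
; Shoot only forwards to the parent implementation.
; Get Socket returns a named socket's transform, name and the SKKA74UX mesh reference.
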(event EventShoot
  (|CallParentFunction))

(fn ConstructionScript
  (|CallParentFunction)
  (bind _output_get (Variables|Default|SetMaxAmmo 45))
  (Variables|Default|SetCurrentAmmo _output_get)
  (Variables|Default|SetMaxDistance 7500)
  (Variables|Default|SetSpread 160)
  (Variables|Default|SetDamage 0.65)
  (Variables|Default|SetFireRate 0.08)
  (Variables|Default|SetKnockback -0.9)
  (Variables|Default|SetFireMode 0) ; 0 - Automatic, 1 - Semi Automatic
  (Variables|Default|SetSoundShoot "/Game/Assets/Sounds/Weapon/AK74_Shoot.AK74_Shoot")
  (Variables|Default|SetSoundNotShoot "/Game/Assets/Sounds/Weapon/Empty.Empty"))

(fn GetSocket
  (params (Socket :type Name :default "None"))
  (bind _sk_ka74u_x (Variables|Default|GetSK_KA74U_X))
  (return (Transformation|GetSocketLocation _sk_ka74u_x Socket) (Transformation|GetSocketRotation _sk_ka74u_x Socket) Socket _sk_ka74u_x))