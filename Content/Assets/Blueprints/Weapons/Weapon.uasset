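; Base weapon actor for the player's ThirdPersonCharacter, handling hitscan firing and reloading from an ammo reserve.
; Shoot checks the character's firing state, looping through Delay in automatic mode or gating CanShoot in semi-automatic.
; AmmoCheck spends a round and calls LineTrace, or plays an empty sound and lengthens the delay.
; LineTrace fires a randomly spread camera trace, applies damage, spawns muzzle effects and adds recoil.
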(event Custom|Shoot
  (bind _self self)
  (bind _soundshoot (Variables|Default|GetSoundShoot))
  (bind _soundnotshoot (Variables|Default|GetSoundNotShoot))
  (bind _firerate (Variables|Default|GetFireRate _self))
  (if (Variables|/Game/Assets/Blueprints/ThirdPersonCharacter.ThirdPersonCharacter_C|GetIsShooting? (.AsThird%20Person%20Character (Utilities|Casting|CastToThirdPersonCharacter (Game|GetPlayerCharacter 0)))) :!label _label
    (if (Variables|Default|GetCanShoot?)
      (switch int (Variables|Default|GetFireMode self) ; 0 - Automatic, 1 - Semi Automatic
        (:0
          (bind _timedelay (CallFunction|AmmoCheck _soundshoot _soundnotshoot))
          (Utilities|FlowControl|Delay (+ _timedelay _firerate))
          (goto _label))
        (:1
          (bind _timedelay_2 (CallFunction|AmmoCheck _soundshoot _soundnotshoot))
          (Variables|Default|SetCanShoot? false)
          (Utilities|FlowControl|Delay (+ _firerate _timedelay_2))
          (Variables|Default|SetCanShoot? true))))))

(event Custom|Reload
  (bind _self self)
  (if (> (- (Variables|Default|GetTotalAmmo _self) (- (Variables|Default|GetMaxAmmo _self) (Variables|Default|GetCurrentAmmo _self))) 0)
    (Variables|Default|SetTotalAmmo _self (- (Variables|Default|GetTotalAmmo _self) (- (Variables|Default|GetMaxAmmo _self) (Variables|Default|GetCurrentAmmo _self))))
    (Variables|Default|SetCurrentAmmo _self (Variables|Default|GetMaxAmmo _self))
    (else
      (Variables|Default|SetCurrentAmmo _self (+ (Variables|Default|GetTotalAmmo _self) (Variables|Default|GetCurrentAmmo _self)))
      (Variables|Default|SetTotalAmmo _self 0))))

(fn ConstructionScript)

(fn AmmoCheck
  (params (SoundShoot :type Sound%20Base%20Object%20Reference) (SoundNotShoot :type Sound%20Base%20Object%20Reference))
  (bind _currentammo (Variables|Default|GetCurrentAmmo))
  (if (Variables|/Game/Assets/Blueprints/ThirdPersonCharacter.ThirdPersonCharacter_C|GetIs%20Can%20Shoot? (.AsThird%20Person%20Character (Utilities|Casting|CastToThirdPersonCharacter (Game|GetPlayerCharacter 0))))
    (if (> _currentammo 0)
      (Math|Integer|DecrementInt _currentammo
        (:%20%20
          (CallFunction|LineTrace)
          (Audio|PlaySoundatLocation SoundShoot (Transformation|GetActorLocation) "0, 0, 0" 1.0 1.0 0.0 0 0 0)
          (return 0.0)))
      (else
        (Audio|PlaySoundatLocation SoundNotShoot (Transformation|GetActorLocation) "0, 0, 0" 1.0 1.0 0.0 0 0 0)
        (return 0.5)))))

(fn LineTrace
  (bind _returnvalue (Game|GetPlayerCameraManager 0))
  (bind _returnvalue_2 (Game|Player|GetPlayerPawn 0))
  (bind _spread (Variables|Default|GetSpread))
  (bind _knockback (Variables|Default|GetKnockback))
  (bind _returnvalue_3 (Camera|GetCameraLocation _returnvalue))
  (bind _returnvalue_4 (* _spread -1))
  (bind _outhit (Collision|LineTraceByChannel _returnvalue_3 (+ (+ _returnvalue_3 (* (Transformation|GetActorForwardVector _returnvalue) (Variables|Default|GetMaxDistance))) (Math|Vector|MakeVector (Math|Conversions|ToFloat(Integer) (Math|Random|RandomIntegerinRange _returnvalue_4 _spread)) (Math|Conversions|ToFloat(Integer) (Math|Random|RandomIntegerinRange _returnvalue_4 _spread)) (Math|Conversions|ToFloat(Integer) (Math|Random|RandomIntegerinRange _returnvalue_4 _spread)))) "TraceTypeQuery1" false 0 "None"))
  (Game|Damage|ApplyDamage (.HitActor (Collision|BreakHitResult _outhit)) (Variables|Default|GetDamage) 0 0)
  (bind (_location _rotation _socketname _objectreference) (Class|BPIGuns|GetSocket(Message) self "Muzzle"))
  (Effects|SpawnEmitterAttached "/Game/InfinityBladeEffects/Shoot1.Shoot1" _objectreference _socketname "0, 0, 0" "0, 0, 0" "0.100000,0.100000,0.100000")
  (Effects|SpawnEmitterAttached "/Game/InfinityBladeEffects/Shoot2.Shoot2" _objectreference _socketname "0, 0, 0" "0, 0, 0" "0.100000,0.100000,0.100000")
  (Effects|SpawnEmitterAttached "/Game/InfinityBladeEffects/Shoot3.Shoot3" _objectreference _socketname "0, 0, 0" "0, 0, 0" "0.100000,0.100000,0.100000")
  (Pawn|Input|AddControllerPitchInput _returnvalue_2 _knockback)
  (Pawn|Input|AddControllerYawInput _returnvalue_2 (Math|Random|RandomFloatinRange _knockback (Math|Float|Absolute(Float) _knockback))))

(fn GetSocket
  (params (Socket :type Name :default "None"))
  (return "0, 0, 0" "0, 0, 0" "None" 0))