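; AK47 weapon Blueprint, a child of a base weapon class that configures an automatic rifle.
; The construction script runs the parent's, then sets ammo, range, spread, damage, fire rate, knockback, fire mode and sounds, starting with a full magazine.
; Shoot defers entirely to the parent implementation.
; GetSocket returns a named socket's location and rotation on the SKKA47 mesh, along with the component reference.
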(event EventShoot
  (|CallParentFunction))

(fn ConstructionScript
  (|CallParentFunction)
  (bind _output_get (Variables|Default|SetMaxAmmo 50))
  (Variables|Default|SetCurrentAmmo _output_get)
  (Variables|Default|SetMaxDistance 7500)
  (Variables|Default|SetSpread 200)
  (Variables|Default|SetDamage 0.5)
  (Variables|Default|SetFireRate 0.1)
  (Variables|Default|SetKnockback -0.7)
  (Variables|Default|SetFireMode 0) ; 0 - Automatic, 1 - Semi Automatic
  (Variables|Default|SetSoundShoot "/Game/Assets/Sounds/Weapon/AK47_Shoot.AK47_Shoot")
  (Variables|Default|SetSoundNotShoot "/Game/Assets/Sounds/Weapon/Empty.Empty"))

(fn GetSocket
  (params (Socket :type Name :default "None"))
  (bind _sk_ka47 (Variables|Default|GetSK_KA47))
  (return (Transformation|GetSocketLocation _sk_ka47 Socket) (Transformation|GetSocketRotation _sk_ka47 Socket) Socket _sk_ka47))