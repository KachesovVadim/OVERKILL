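; AR4 weapon Blueprint, an automatic assault rifle that extends a parent weapon class.
; Its construction script runs the parent's, then sets the rifle's ammo, range, spread, damage, fire rate, knockback and sounds.
; The Shoot event defers entirely to the parent, and Get Socket returns a named socket's location, rotation and the SKAR4 component.
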(event EventShoot
  (|CallParentFunction))

(fn ConstructionScript
  (|CallParentFunction)
  (bind _output_get (Variables|Default|SetMaxAmmo 40))
  (Variables|Default|SetCurrentAmmo _output_get)
  (Variables|Default|SetMaxDistance 7500)
  (Variables|Default|SetSpread 150)
  (Variables|Default|SetDamage 0.7)
  (Variables|Default|SetFireRate 0.12)
  (Variables|Default|SetKnockback -0.8)
  (Variables|Default|SetFireMode 0) ; 0 - Automatic, 1 - Semi Automatic
  (Variables|Default|SetSoundShoot "/Game/Assets/Sounds/Weapon/AR4_Shoot.AR4_Shoot")
  (Variables|Default|SetSoundNotShoot "/Game/Assets/Sounds/Weapon/Empty.Empty"))

(fn GetSocket
  (params (Socket :type Name :default "None"))
  (bind _sk_ar4 (Variables|Default|GetSK_AR4))
  (return (Transformation|GetSocketLocation _sk_ar4 Socket) (Transformation|GetSocketRotation _sk_ar4 Socket) Socket _sk_ar4))