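; BoxTeleport is an actor that teleports any actor overlapping it to a Destination, resetting its rotation to zero.
; Each teleport spawns a Portal particle system at the box and another at the destination, which uses its own rotation variable.
; As a fallback, Tick polls for overlapping Zombie actors and sends any still inside through the same teleport and effects via a custom Overlap event.
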(event Custom|Overlap
  (params (Other%20Actor :type Actor%20Object%20Reference))
  (bind _destination (Variables|Default|GetDestination))
  (Transformation|Teleport Other%20Actor _destination "0, 0, 0")
  (Niagara|SpawnSystematLocation "/Game/Assets/Portal/Portal.Portal" (Transformation|GetActorLocation) (Transformation|GetActorRotation)) ; Portal at spawn
  (Niagara|SpawnSystematLocation "/Game/Assets/Portal/Portal.Portal" _destination (Variables|Default|GetDestinationRoration)) ; Portal at destination
)

(event Collision|EventActorBeginOverlap
  (params (OtherActor :type Actor%20Object%20Reference))
  (bind _destination (Variables|Default|GetDestination))
  (Transformation|Teleport OtherActor _destination "0, 0, 0")
  (Niagara|SpawnSystematLocation "/Game/Assets/Portal/Portal.Portal" (Transformation|GetActorLocation) (Transformation|GetActorRotation)) ; Portal at spawn
  (Niagara|SpawnSystematLocation "/Game/Assets/Portal/Portal.Portal" _destination (Variables|Default|GetDestinationRoration)) ; Portal at destination
)

(event EventTick
  (params (DeltaSeconds :type Float%20%28single-precision%29))
  (bind _overlappingactors (Collision|GetOverlappingActors "/Game/Assets/Blueprints/Enemies/Zombie.Zombie_C" :!class /Script/Engine.Actor))
  (if (Utilities|Array|IsValidIndex _overlappingactors)
    (for _array_element _overlappingactors
      (CallFunction|Overlap _array_element) ; If the zombie overlapped, but didnt teleport
    )))

(fn ConstructionScript)