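; AcornBP is a spinning acorn pickup that sets the player character's Health on overlap.
; BeginPlay spawns an Acorn particle emitter below the actor, and Tick increments roll and yaw by a fixed, frame-rate-dependent step.
; When the player overlaps it, Health is set to half on the first level or full otherwise, then the emitter is removed, a sound plays and the actor destroys itself.
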(event EventBeginPlay
  (bind _returnvalue (Transformation|GetActorLocation))
  (bind _returnvalue_2 (Effects|SpawnEmitteratLocation "/Game/InfinityBladeEffects/Acorn.Acorn" (Math|Vector|MakeVector (.x _returnvalue) (.y _returnvalue) (+ (.z _returnvalue) -2e+02)))))

(event Collision|EventActorBeginOverlap
  (params (OtherActor :type Actor%20Object%20Reference))
  (bind _returnvalue (Game|GetPlayerCharacter 0))
  (bind _asthird_person_character (Utilities|Casting|CastToThirdPersonCharacter _returnvalue))
  (if (== OtherActor _asthird_person_character)
    (if (== (Variables|/Game/Assets/Blueprints/ThirdPersonCharacter.ThirdPersonCharacter_C|GetCurrentLevel _asthird_person_character) 0) ; If current level 1
      (Variables|/Game/Assets/Blueprints/ThirdPersonCharacter.ThirdPersonCharacter_C|SetHealth _asthird_person_character 0.5)
      (else
        (Variables|/Game/Assets/Blueprints/ThirdPersonCharacter.ThirdPersonCharacter_C|SetHealth _asthird_person_character 1.0)))
    (Components|DestroyComponent (stale EventBeginPlay _returnvalue_2))
    (Audio|PlaySoundatLocation "/Game/Assets/Sounds/AcornPickup.AcornPickup" (Transformation|GetActorLocation) "0, 0, 0" 1.0 1.0 0.0 0 0 0)
    (Actor|DestroyActor)))

(event EventTick
  (params (DeltaSeconds :type Float%20%28single-precision%29))
  (bind _returnvalue (Transformation|GetActorRotation))
  (Transformation|SetActorRotation (Math|Rotator|MakeRotator (+ (.roll _returnvalue) 1.0) 0.0 (+ (.yaw _returnvalue) 1.0))))

(fn ConstructionScript)