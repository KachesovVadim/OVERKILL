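; Zombie enemy that chases and attacks the player, with damage, health, speed and acorn drop odds adjusted by the player's level settings.
; A delayed self-calling loop runs AI MoveTo, halts for montage attacks up close, and periodically destroys zombies stuck in place.
; Lethal damage triggers ragdoll; the loop then awards money, updates the player's zombie count, checks for a win and may drop an acorn.
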(event Custom|Spawned
  (bind _returnvalue (Game|GetPlayerCharacter 0))
  (bind _asthird_person_character (Utilities|Casting|CastToThirdPersonCharacter _returnvalue))
  (bind _asthird_person_character_2 (Utilities|Casting|CastToThirdPersonCharacter (Game|GetPlayerCharacter 0)))
  (Variables|Default|SetCharacterReference _asthird_person_character_2)
  (Variables|/Script/Engine.CharacterMovementComponent|SetMaxWalkSpeed (Variables|Character|GetCharacterMovement) (* (Variables|Default|GetSpeedMulti) (Utilities|Select :Index (Math|Random|RandomInteger 3) :Option%200 5e+02 :Option%201 5.5e+02 :Option%202 6e+02 :Option%203 6.5e+02)))
  (Audio|SpawnSoundatLocation "/Game/Assets/Sounds/Enemies/Zombie/ZombieSpawn.ZombieSpawn" (Transformation|GetActorLocation) "0, 0, 0" 1.0 1.0 0.0 "/Game/Assets/Sounds/SoundAttenuation.SoundAttenuation" 0)
  (Variables|/Game/Assets/Blueprints/ThirdPersonCharacter.ThirdPersonCharacter_C|SetTotalZombies _asthird_person_character (+ (Variables|/Game/Assets/Blueprints/ThirdPersonCharacter.ThirdPersonCharacter_C|GetTotalZombies _asthird_person_character) 1))
  (CallFunction|FollowtoCharacter))

(event Custom|FollowToCharacter
  (bind _returnvalue (Game|GetPlayerCharacter 0))
  (bind _returnvalue_2 (Transformation|GetActorLocation))
  (bind _asthird_person_character (Utilities|Casting|CastToThirdPersonCharacter _returnvalue))
  (if (Variables|Default|GetIsDead)
    (Variables|/Game/Assets/Blueprints/ThirdPersonCharacter.ThirdPersonCharacter_C|SetMoney _asthird_person_character (+ (Variables|/Game/Assets/Blueprints/ThirdPersonCharacter.ThirdPersonCharacter_C|GetMoney _asthird_person_character) 100))
    (Collision|SetCollisionEnabled (Variables|Collision|GetCapsuleComponent) "NoCollision")
    (Variables|/Game/Assets/Blueprints/ThirdPersonCharacter.ThirdPersonCharacter_C|SetTotalZombies _asthird_person_character (- (Variables|/Game/Assets/Blueprints/ThirdPersonCharacter.ThirdPersonCharacter_C|GetTotalZombies _asthird_person_character) 1))
    (Default|CheckWin _asthird_person_character)
    ;[1 1 1] Gold Accorn
    (if (== (Math|Random|RandomIntegerinRange 0 (Variables|Default|GetMaxAccornRange)) 1)
      (Game|SpawnActorfromClass "/Game/Assets/Blueprints/Acorn/AcornBP.AcornBP_C" (Math|Transform|MakeTransform (Math|Vector|MakeVector (.x _returnvalue_2) (.y _returnvalue_2) (+ (.z _returnvalue_2) 1e+02)) "0, 0, 0" "1,1,1") "Undefined" 0 0))
    (Utilities|FlowControl|Delay 1e+01)
    (Actor|DestroyActor)
    (elif (>= (Variables|Default|GetStuckPoints) 50)
      (CallFunction|CheckStuck)
      (else
        (if (>= (Transformation|GetDistanceTo (Variables|Default|GetCharacterReference)) 2e+02)
          (AI|AIMoveTo self "0, 0, 0" (Variables|Default|GetCharacterReference) 0.0 false
            (:then
              _))
          (else
            (CallFunction|Attack)
            (if (Variables|Default|GetHitEnd) :!label _label
              _
              (else
                (Utilities|FlowControl|Delay 0.1)
                (goto _label)))))
        (Utilities|FlowControl|Delay 0.2)
        (Variables|Default|SetStuckPoints (+ (Variables|Default|GetStuckPoints) 1)) ; If this points = 50, check stuck
        (CallFunction|FollowtoCharacter)))))

(event Custom|Attack
  (bind _charactermovement (Variables|Character|GetCharacterMovement))
  (if (!= (Variables|/Script/Engine.CharacterMovementComponent|GetMaxWalkSpeed _charactermovement) 0.0)
    (Variables|Default|SetTempSpeed (Variables|/Script/Engine.CharacterMovementComponent|GetMaxWalkSpeed _charactermovement))
    (Variables|/Script/Engine.CharacterMovementComponent|SetMaxWalkSpeed _charactermovement 0.0))
  (Animation|PlayAnimMontage "/Game/Assets/Enemies/Zombie/Animations/Zombie_Attack_Montage.Zombie_Attack_Montage" 1.0 "None")
  (Variables|Default|SetHitEnd false))

(event Custom|CheckStuck
  (bind _returnvalue (Game|GetPlayerCharacter 0))
  (bind _charactermovement (Variables|Character|GetCharacterMovement))
  (bind _returnvalue_2 (Class|PawnMovementComponent|GetPawnOwner _charactermovement))
  (bind _asthird_person_character (Utilities|Casting|CastToThirdPersonCharacter _returnvalue))
  (bind _returnvalue_3 (Transformation|GetActorLocation _returnvalue_2))
  (if (Math|Vector|Equal(Vector) _returnvalue_3 (Variables|Default|GetPos) 5e+01)
    (if (== (Variables|/Script/Engine.CharacterMovementComponent|GetMaxWalkSpeed (Variables|Character|GetCharacterMovement)) 0.0) ; If attack
      (Variables|Default|SetPos _returnvalue_3 :!label _label)
      (Variables|Default|SetStuckPoints 0)
      (CallFunction|FollowtoCharacter)
      (else
        (Actor|DestroyActor)
        (Variables|/Game/Assets/Blueprints/ThirdPersonCharacter.ThirdPersonCharacter_C|SetTotalZombies _asthird_person_character (- (Variables|/Game/Assets/Blueprints/ThirdPersonCharacter.ThirdPersonCharacter_C|GetTotalZombies _asthird_person_character) 1))
        (Default|CheckWin _asthird_person_character)))
    (else
      (goto _label))))

(event EventBeginPlay
  (switch int (Math|Float|Truncate (Utilities|Array|Get(acopy) (Variables|/Game/Assets/Blueprints/ThirdPersonCharacter.ThirdPersonCharacter_C|GetLevelSpecifics (.AsThird%20Person%20Character (Utilities|Casting|CastToThirdPersonCharacter (Game|GetPlayerCharacter 0)))) 1))
    (:Default
      _)
    (:2
      (Variables|Default|SetDamage (* (Variables|Default|GetDamage) 3.0))
      (Variables|Default|SetHealth 1.2))
    (:3
      (Variables|Default|SetDamage (* (Variables|Default|GetDamage) 2.0))
      (Variables|Default|SetSpeedMulti 2.0)
      (Variables|Default|SetHealth 2.0))
    (:4
      _)
    (:5
      (Variables|Default|SetMaxAccornRange 100)
      (Variables|Default|SetSpeedMulti 1.5)))
  (CallFunction|Spawned))

(event Game|Damage|EventAnyDamage
  (params (Damage :type Float%20%28single-precision%29) (DamageType :type Damage%20Type%20Object%20Reference) (InstigatedBy :type Controller%20Object%20Reference) (DamageCauser :type Actor%20Object%20Reference))
  (CallFunction|TakeDamage Damage true))

(fn ConstructionScript)

(fn TakeDamage
  (params (Damage :type Float%20%28single-precision%29) (SoundOn? :type Boolean))
  (if (not (Variables|Default|GetIsDead))
    (if SoundOn?
      (Audio|PlaySoundatLocation (Utilities|Select :Index (Math|Random|RandomInteger 2) :Option%200 "/Game/Assets/Enemies/HitSounds/hit1.hit1" :Option%201 "/Game/Assets/Enemies/HitSounds/hit2.hit2" :Option%202 "/Game/Assets/Enemies/HitSounds/hit3.hit3") (Transformation|GetActorLocation) "0, 0, 0" 1.0 1.0 0.0 0 0 0))
    (bind _output_get (Variables|Default|SetHealth (- (Variables|Default|GetHealth) Damage)))
    (if (not (> _output_get 0.0))
      (Pawn|Components|CharacterMovement|DisableMovement (Variables|Character|GetCharacterMovement))
      (Physics|SetSimulatePhysics (Variables|Character|GetMesh) true)
      (Variables|Default|SetIsDead true))))