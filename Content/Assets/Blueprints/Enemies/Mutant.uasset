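; Mutant boss enemy that chases the player and melee attacks, driving the boss health bar on the player's BossFightHUD.
; A self-recalling FollowToCharacter loop moves toward the player or, within range, halts, plays an attack montage and polls HitEnd, which is set true elsewhere.
; TakeDamage plays hit sounds and ragdolls the mutant at zero health; the loop then plays the death sound, removes the HUD and calls LevelEnd.
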(event Custom|Spawned
  (bind _asthird_person_character (Utilities|Casting|CastToThirdPersonCharacter (Game|GetPlayerCharacter 0)))
  (Variables|Default|SetCharacterReference _asthird_person_character)
  (Variables|/Script/Engine.CharacterMovementComponent|SetMaxWalkSpeed (Variables|Character|GetCharacterMovement) 1e+03)
  (Audio|SpawnSoundatLocation 0 (Transformation|GetActorLocation) "0, 0, 0" 1.0 1.0 0.0 "/Game/Assets/Sounds/SoundAttenuation.SoundAttenuation" 0)
  (Utilities|FlowControl|Delay 0.05)
  (Variables|/Game/Assets/HUDS/BossFight.BossFight_C|SetBossHealth (Variables|/Game/Assets/Blueprints/ThirdPersonCharacter.ThirdPersonCharacter_C|GetBossFightHUD (Variables|Default|GetCharacterReference)) (/ (Variables|Default|GetHealth) 2e+03))
  (CallFunction|FollowtoCharacter))

(event Custom|FollowToCharacter
  (bind _characterreference (Variables|Default|GetCharacterReference))
  (if (Variables|Default|GetIsDead)
    (Collision|SetCollisionEnabled (Variables|Collision|GetCapsuleComponent) "NoCollision")
    (Audio|SpawnSoundatLocation "/Game/Assets/Sounds/Enemies/Mutant/MutantDeath.MutantDeath" (Transformation|GetActorLocation) "0, 0, 0" 1.0 1.0 0.0 "/Game/Assets/Sounds/SoundAttenuation.SoundAttenuation" 0)
    (Utilities|FlowControl|Delay 3.0)
    (Widget|RemovefromParent (Variables|/Game/Assets/Blueprints/ThirdPersonCharacter.ThirdPersonCharacter_C|GetBossFightHUD _characterreference))
    (Default|LevelEnd _characterreference false)
    (else
      (if (>= (Transformation|GetDistanceTo (Variables|Default|GetCharacterReference)) 2e+02)
        (AI|AIMoveTo self "0, 0, 0" (Variables|Default|GetCharacterReference) 0.0 false
          (:then
            _))
        (else
          (CallFunction|Attack)
          (if (Variables|Default|GetHitEnd) :!label _label
            _
            (else
              (Utilities|FlowControl|Delay 0.1)
              (goto _label)))))
      (Utilities|FlowControl|Delay 0.2)
      (CallFunction|FollowtoCharacter))))

(event Custom|Attack
  (bind _charactermovement (Variables|Character|GetCharacterMovement))
  (if (!= (Variables|/Script/Engine.CharacterMovementComponent|GetMaxWalkSpeed _charactermovement) 0.0)
    (Variables|Default|SetTempSpeed (Variables|/Script/Engine.CharacterMovementComponent|GetMaxWalkSpeed _charactermovement))
    (Variables|/Script/Engine.CharacterMovementComponent|SetMaxWalkSpeed _charactermovement 0.0))
  (Animation|PlayAnimMontage (Utilities|Select :Index (Math|Random|RandomInteger 1) :Option%200 "/Game/Assets/Enemies/MutantBoss/Animations/Attack1_Montage.Attack1_Montage" :Option%201 "/Game/Assets/Enemies/MutantBoss/Animations/Attack2_Montage.Attack2_Montage") 1.0 "None")
  (Variables|Default|SetHitEnd false))

(event Game|Damage|EventAnyDamage
  (params (Damage :type Float%20%28single-precision%29) (DamageType :type Damage%20Type%20Object%20Reference) (InstigatedBy :type Controller%20Object%20Reference) (DamageCauser :type Actor%20Object%20Reference))
  (Variables|/Game/Assets/HUDS/BossFight.BossFight_C|SetBossHealth (Variables|/Game/Assets/Blueprints/ThirdPersonCharacter.ThirdPersonCharacter_C|GetBossFightHUD (Variables|Default|GetCharacterReference)) (/ (Variables|Default|GetHealth) 2e+03))
  (CallFunction|TakeDamage Damage true))

(fn ConstructionScript)

(fn TakeDamage
  (params (Damage :type Float%20%28single-precision%29) (SoundOn? :type Boolean))
  (if (not (Variables|Default|GetIsDead))
    (if SoundOn?
      (Audio|PlaySoundatLocation (Utilities|Select :Index (Math|Random|RandomInteger 2) :Option%200 "/Game/Assets/Enemies/HitSounds/hit1.hit1" :Option%201 "/Game/Assets/Enemies/HitSounds/hit2.hit2" :Option%202 "/Game/Assets/Enemies/HitSounds/hit3.hit3") (Transformation|GetActorLocation) "0, 0, 0" 1.0 1.0 0.0 0 0 0))
    (bind _output_get (Variables|Default|SetHealth (- (Variables|Default|GetHealth) Damage)))
    (if (not (> _output_get 0.0))
      (Pawn|Components|CharacterMovement|DisableMovement (Variables|Character|GetCharacterMovement))
      (Physics|SetSimulatePhysics (Variables|Character|GetMesh) true)
      (Variables|Default|SetIsDead true))))